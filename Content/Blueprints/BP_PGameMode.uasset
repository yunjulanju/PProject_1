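; Game mode that runs a 180-second timed round, keeping BP_Monster actors populated around a center point.
; Tick accumulates elapsed time, prints it against the limit, and spawns one monster at a random XY offset from CenterVector whenever the count is at or below MonsterNum.
; Once time is up, Tick destroys all monsters, printing a Korean game-over message for each.
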(event EventBeginPlay)

(event EventTick
  (params (DeltaSeconds :type Float%20%28single-precision%29))
  (bind _returnvalue (Math|Random|RandomFloatinRange -2e+03 2e+03))
  (bind _centervector (Variables|Default|GetCenterVector))
  (bind _output_get (Variables|Default|SetSum%20Time (+ DeltaSeconds (Variables|Default|GetSum%20Time))))
  (Development|PrintString (Utilities|String|ToString(Text) (Utilities|Text|FormatText "현재 시간 : {1} / 제한시간 : 180.0" _output_get)) true true "(R=0.000000,G=0.660000,B=1.000000,A=1.000000)" 0.0)
  (if (>= (Variables|Default|GetSum%20Time) 1.8e+02)
    (bind _outactors (Actor|GetAllActorsOfClass "/Game/Blueprints/Monster/BP_Monster.BP_Monster_C"))
    (for _array_element _outactors
      (Actor|DestroyActor _array_element)
      (Development|PrintString "게임 종료" true true "(R=1.000000,G=0.027441,B=0.000000,A=1.000000)" 5.0))
    (else
      (bind _outactors_2 (Actor|GetAllActorsOfClass "/Game/Blueprints/Monster/BP_Monster.BP_Monster_C"))
      (if (<= (Utilities|Array|Length _outactors_2) (Variables|Default|GetMonsterNum))
        (Game|SpawnActorfromClass "/Game/Blueprints/Monster/BP_Monster.BP_Monster_C" (Math|Transform|MakeTransform (Math|Vector|MakeVector (+ (.x _centervector) _returnvalue) (+ (.y _centervector) _returnvalue) (.z _centervector)) "0, 0, 0" "1.000000,1.000000,1.000000") "Undefined" "MultiplyWithRoot" 0 0)))))

(fn ConstructionScript)