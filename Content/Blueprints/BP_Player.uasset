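; Player Blueprint that tracks health and handles hitscan shooting at monsters.
; HP starts at MaxHP and prints on screen each tick, while Fire plays the firing montage.
; Shot traces from screen center to find an aim point, then from the given mesh socket toward it.
; A BP_Monster hit plays a roar at world origin and subtracts AP from its HP, calling Damage only when HP reaches zero.
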(event EventBeginPlay
  (Variables|Default|SetHP (Variables|Default|GetMaxHP)))

(event Collision|EventActorBeginOverlap
  (params (OtherActor :type Actor%20Object%20Reference)))

(event EventTick
  (params (DeltaSeconds :type Float%20%28single-precision%29))
  (Development|PrintString (Utilities|String|ToString(Text) (Utilities|Text|FormatText "플레이어 체력 : {0}" (Variables|Default|GetHP))) true true "(R=0.000000,G=1.000000,B=0.155178,A=1.000000)" 0.0))

(fn ConstructionScript)

(fn Fire
  (Animation|PlayAnimMontage "/Game/Animations/AM_Fire.AM_Fire" 1.0 "None"))

(fn Shot
  (params (SocketName :type Name))
  (bind _returnvalue (Viewport|GetViewportSize))
  (bind _returnvalue_2 (Game|GetPlayerController 0))
  (bind _returnvalue_3 (/ (.x _returnvalue) 2.0))
  (bind _returnvalue_4 (/ (.y _returnvalue) 2.0))
  (bind (_worldposition _worlddirection) (Class|GameplayStatics|DeprojectScreentoWorld _returnvalue_2 (Math|Vector2D|MakeVector2D _returnvalue_3 _returnvalue_4)))
  (bind (_outhit _returnvalue_5) (Collision|LineTraceByChannel _worldposition (+ _worldposition (* _worlddirection 1e+04)) "TraceTypeQuery1" false 0 "None" true "(R=1.000000,G=0.000000,B=0.000000,A=1.000000)" "(R=0.000000,G=1.000000,B=0.000000,A=1.000000)" 1.0))
  (if _returnvalue_5
    (bind _outhit_2 (Collision|LineTraceByChannel (.location (Transformation|GetSocketTransform (Variables|Character|GetMesh) SocketName "RTS_World")) (.Location (Collision|BreakHitResult _outhit)) "TraceTypeQuery1" false 0 "None" true "(R=0.477455,G=0.017945,B=1.000000,A=1.000000)" "(R=1.000000,G=0.692639,B=0.000000,A=1.000000)" 1.0))
    (bind _asbp_monster (Utilities|Casting|CastToBP_Monster (.HitActor (Collision|BreakHitResult _outhit_2))))
    (Utilities|IsValid _asbp_monster
      (:Is%20Valid
        (Audio|PlaySoundatLocation "/Game/MonsterRoarsAndGrowls/wav/04_Signal_Roar.04_Signal_Roar" "0, 0, 0" "0, 0, 0" 1.0 1.0 0.0 0 0 0 0)
        (if (> (Variables|/Game/Blueprints/Monster/BP_Monster.BP_Monster_C|GetHP _asbp_monster) 0.0)
          (if (<= (- (Variables|/Game/Blueprints/Monster/BP_Monster.BP_Monster_C|GetHP _asbp_monster) (Variables|Default|GetAP)) 0.0)
            (Variables|/Game/Blueprints/Monster/BP_Monster.BP_Monster_C|SetHP _asbp_monster 0.0)
            (Default|Damage _asbp_monster)
            (else
              (Variables|/Game/Blueprints/Monster/BP_Monster.BP_Monster_C|SetHP _asbp_monster (- (Variables|/Game/Blueprints/Monster/BP_Monster.BP_Monster_C|GetHP _asbp_monster) (Variables|Default|GetAP)))
              (Development|PrintString (Utilities|String|ToString(Text) (Utilities|Text|FormatText "몬스터의 체력 : {0}" (Variables|/Game/Blueprints/Monster/BP_Monster.BP_Monster_C|GetHP _asbp_monster))) true true "(R=0.125258,G=0.000000,B=1.000000,A=1.000000)" 1.0))))))))