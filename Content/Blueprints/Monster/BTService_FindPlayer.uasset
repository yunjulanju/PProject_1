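; Behavior tree service for monster AI that decides whether to chase the player based on distance.
; On activation it waits briefly, then caches the first BP_Player actor found in the level.
; Each tick it measures the distance from the controlled pawn to that player.
; Within a fixed radius it sets the chasing flag and Player blackboard keys, otherwise it clears both.
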(event EventReceiveTickAI
  (params (OwnerController :type AI%20Controller%20Object%20Reference) (ControlledPawn :type Pawn%20Object%20Reference) (DeltaSeconds :type Float%20%28single-precision%29))
  (bind _bpplayer (Variables|Default|GetBPPlayer))
  (Utilities|IsValid _bpplayer
    (:Is%20Valid
      (if (> (Math|Vector|VectorLength (- (Transformation|GetActorLocation _bpplayer) (Transformation|GetActorLocation ControlledPawn))) 5e+02)
        (Class|BTFunctionLibrary|SetBlackboardValueasBool (Variables|Default|GetbIsChasing) false)
        (Class|BTFunctionLibrary|SetBlackboardValueasObject (Variables|Default|GetPlayer))
        (else
          (Class|BTFunctionLibrary|SetBlackboardValueasBool (Variables|Default|GetbIsChasing) true)
          (Class|BTFunctionLibrary|SetBlackboardValueasObject (Variables|Default|GetPlayer) (Variables|Default|GetBPPlayer)))))))

(event EventReceiveActivationAI
  (params (OwnerController :type AI%20Controller%20Object%20Reference) (ControlledPawn :type Pawn%20Object%20Reference))
  (Utilities|FlowControl|Delay 0.2)
  (bind _returnvalue (Actor|GetActorOfClass "/Game/Blueprints/BP_Player.BP_Player_C"))
  (Variables|Default|SetBPPlayer _returnvalue))